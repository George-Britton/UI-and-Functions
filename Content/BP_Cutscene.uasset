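; BP_Cutscene is a short cutscene actor that flies its camera along a spline, then hands back to the third-person character.
; Tick accumulates elapsed time and teleports the camera to the matching spline position in world space, without constant velocity.
; BeginPlay activates the camera, waits three seconds, activates the FollowCamera on BP_ThirdPersonCharacter and destroys the actor.
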(event EventTick
  (params (DeltaSeconds :type Float%20%28single-precision%29))
  (Variables|Default|SetTime (+ DeltaSeconds (Variables|Default|GetTime)))
  (Transformation|SetWorldLocation (Variables|Default|GetCamera) (Spline|GetLocationatTime (Variables|Default|GetSpline) (Variables|Default|GetTime) "World" false) false true))

(event EventBeginPlay
  (Components|Activation|SetActive (Variables|Default|GetCamera) true false)
  (Utilities|FlowControl|Delay 3.0)
  (bind _returnvalue (Actor|GetActorOfClass "/Game/ThirdPerson/Blueprints/BP_ThirdPersonCharacter.BP_ThirdPersonCharacter_C"))
  (Components|Activation|SetActive (Variables|/Game/ThirdPerson/Blueprints/BP_ThirdPersonCharacter.BP_ThirdPersonCharacter_C|GetFollowCamera _returnvalue) true false)
  (Actor|DestroyActor))

(fn ConstructionScript)