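; BP_Tree is a tree actor exposing functions to set its mesh, material, height and mesh component, plus return a partly populated secret struct.
; SetMesh adds a static mesh component when TreeMesh is invalid; SetHeight clamps Z scale.
; AnyDamage ignores Blueprint_Effect_Fire damage, otherwise overwrites Health with clamped damage rather than subtracting it, printing a debug string at zero.
; The node resetting Health to full is unconnected.
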(event Game|Damage|EventAnyDamage
  (params (Damage :type Float%20%28single-precision%29) (DamageType :type Damage%20Type%20Object%20Reference) (InstigatedBy :type Controller%20Object%20Reference) (DamageCauser :type Actor%20Object%20Reference))
  (bind _returnvalue (Math|Float|Clamp(Float) Damage 0.0 1e+02))
  (if (not (== DamageType "/Game/StarterContent/Blueprints/Blueprint_Effect_Fire.Blueprint_Effect_Fire"))
    (Variables|Default|SetHealth _returnvalue)
    (if (== _returnvalue 0.0)
      (Development|PrintString "ded"))))

(fn ConstructionScript)

(fn ChangeColour
  (params (Colour :type Material%20Object%20Reference))
  (Utilities|IsValid (Variables|/Script/Engine.StaticMeshComponent|GetStaticMesh (Variables|Default|GetTreeMesh))
    (:Is%20Valid
      (Rendering|Material|SetMaterial (Variables|Default|GetTreeMesh) 0 Colour)
      (return true))
    (:Is%20Not%20Valid
      (return false))))

(fn SetHeight
  (params (NewHeight :type Float%20%28double-precision%29))
  (bind _returnvalue (Transformation|GetActorScale3D))
  (Transformation|SetActorScale3D (Math|Vector|MakeVector (.x _returnvalue) (.y _returnvalue) (Math|Float|Clamp(Float) NewHeight 0.5 1e+01)))
  (return (.z (Transformation|GetActorScale3D))))

(fn SetTreeComp
  (params (NewTreeComp :type Primitive%20Component%20Object%20Reference))
  (bind _asstatic_mesh_component (Utilities|Casting|CastToStaticMeshComponent NewTreeComp)
    (:then
      (Variables|Default|SetTreeMesh _asstatic_mesh_component)
      (return true))
    (:CastFailed
      (Utilities|String|LogString "That's not a static mesh comp you fool")
      (return false))))

(fn GetSecret
  (bind _secret (Variables|Default|GetSecret))
  (bind _output_get (LocalVariables|SetTempSecret (Utilities|Struct|MakePyTestStruct (.bool _secret) 0 0.0 "One" "-------" (.name _secret) "" 0 0 0)))
  (return _output_get))

(fn SetMesh
  (params (StaticMesh :type Static%20Mesh%20Object%20Reference))
  (Utilities|IsValid (Variables|Default|GetTreeMesh)
    (:Is%20Valid
      (Components|StaticMesh|SetStaticMesh (Variables|Default|GetTreeMesh) StaticMesh)
      (return))
    (:Is%20Not%20Valid
      (bind _returnvalue (Game|AddComponentbyClass "/Script/Engine.StaticMeshComponent" false))
      (bind _output_get (Variables|Default|SetTreeMesh _returnvalue))
      (Components|StaticMesh|SetStaticMesh _output_get StaticMesh)
      (return))))