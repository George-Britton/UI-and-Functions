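; BP_TreeManager is a manager actor that sets the height of the BP_Tree actors in the world when play begins.
; On BeginPlay it caches every BP_Tree into a Trees array, then SetTreeHeight loops over them, calling SetHeight with one fixed value.
; It stores each returned height and prints an error message if that height exceeds the requested value.
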(event EventBeginPlay
  (bind _outactors (Actor|GetAllActorsOfClass "/Game/BP_Tree.BP_Tree_C"))
  (Variables|Default|SetTrees _outactors)
  (CallFunction|SetTreeHeight))

(event Collision|EventActorBeginOverlap
  (params (OtherActor :type Actor%20Object%20Reference)))

(event EventTick
  (params (DeltaSeconds :type Float%20%28single-precision%29)))

(fn ConstructionScript)

(fn SetTreeHeight
  (for _array_element (Variables|Default|GetTrees)
    (bind _setheight (Default|SetHeight _array_element 5e+03))
    (bind _output_get (LocalVariables|SetNewTreeHeight _setheight))
    (if (> _output_get 5e+03)
      (Development|PrintString "Something went wrong")))
  (return))